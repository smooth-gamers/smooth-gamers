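; Level-exit elevator that moves the player to the next level when they enter its trigger box.
; On a player overlap it plays a ding, gets the new level from the game manager using the current one, then calls NextLevel.
; At BeginPlay only, it colours the cube inactive or active based on the manager's enemy count.
; The overlap itself does not check remaining enemies.
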(event `self.Box.OnComponentBeginOverlap`
  (params (OverlappedComponent :type "PrimitiveComponent Object Reference") (OtherActor :type "Actor Object Reference") (OtherComp :type "PrimitiveComponent Object Reference") (OtherBodyIndex :type Integer) (bFromSweep :type Boolean) (SweepResult :type "HitResult Structure (by ref)"))
  (bind _mygamemanager (`/Game/PublicStuff/MyFunctionLibrary.GetMyGameManager`))
  (if (`self.ActorHasTag` OtherActor "Player_Tag")
    (cast `/Game/FirstPersonBP/Blueprints/FirstPersonCharacter` OtherActor)
    (`GameplayStatics.PlaySoundAtLocation` "/Game/Bailey/Sounds/Elevator_Ding.Elevator_Ding" (`self.K2_GetActorLocation`) (struct) 1.0 1.0 0.0 null null null) ; Play firing sound
    (bind _new_level (`/Game/PublicStuff/MyGameManager.Change Level Variable` _mygamemanager (`/Game/PublicStuff/MyGameManager.Current Level` _mygamemanager)))
    (bind _output_get (set `/Game/PublicStuff/MyGameManager.New Level` _new_level _mygamemanager))
    (`/Game/PublicStuff/MyGameManager.Next Level` _mygamemanager _output_get)))

(event `self.ReceiveBeginPlay`
  (`self.Elevator Colour`))

(fn `Elevator Colour`
  (bind _cube (`self.Cube`))
  (bind _mygamemanager (`/Game/PublicStuff/MyFunctionLibrary.GetMyGameManager`))
  (if (>= (`/Game/PublicStuff/MyGameManager.Enemies` _mygamemanager) 1)
    (`PrimitiveComponent.SetMaterial` _cube 0 "/Game/Logain/ElevatorInactive_Mat.ElevatorInactive_Mat")
    (else
      (`PrimitiveComponent.SetMaterial` _cube 0 "/Game/Logain/ElevatorActive_Mat.ElevatorActive_Mat"))))

(fn `UserConstructionScript`)