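; BP_Lasers is a laser hazard that changes the health of a player-tagged FirstPersonCharacter inside its capsule.
; The construction script shifts the capsule along world Z and adds to its Z scale using length and scale variables.
; Entry resets accumulated damage to InstantDamage, but applies it only when it exceeds MaxDamage, clamped to that limit.
; While the player stays inside, Tick applies DamageRate over time until the accumulated total reaches MaxDamage.
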(event `self.ReceiveTick`
  (params (DeltaSeconds :type "Float (single-precision)"))
  (if (`self.Inside Volume`)
    (`self.Continue Damage`)))

(event `self.Capsule.OnComponentBeginOverlap`
  (params (OverlappedComponent :type "PrimitiveComponent Object Reference") (OtherActor :type "Actor Object Reference") (OtherComp :type "PrimitiveComponent Object Reference") (OtherBodyIndex :type Integer) (bFromSweep :type Boolean) (SweepResult :type "HitResult Structure (by ref)"))
  (if (`self.ActorHasTag` OtherActor "Player_Tag")
    (bind _asfirst_person_character (cast `/Game/FirstPersonBP/Blueprints/FirstPersonCharacter` OtherActor))
    (set `self.Inside Volume` true)
    (set `self.Player` _asfirst_person_character)
    (`self.Start Damage`)))

(event `self.Capsule.OnComponentEndOverlap`
  (params (OverlappedComponent :type "PrimitiveComponent Object Reference") (OtherActor :type "Actor Object Reference") (OtherComp :type "PrimitiveComponent Object Reference") (OtherBodyIndex :type Integer))
  (if (`self.ActorHasTag` OtherActor "Player_Tag")
    (cast `/Game/FirstPersonBP/Blueprints/FirstPersonCharacter` OtherActor)
    (set `self.Inside Volume` false)))

(fn `Continue Damage`
  (bind _returnvalue (* (`self.Damage Rate`) (`GameplayStatics.GetWorldDeltaSeconds`)))
  (if (< (`self.Accum Damage`) (`self.Max Damage`))
    (set `self.Accum Damage` (+ (`self.Accum Damage`) _returnvalue))
    (`/Game/FirstPersonBP/Blueprints/FirstPersonCharacter.Change Health` (`self.Player`) _returnvalue)))

(fn `Start Damage`
  (bind _output_get (set `self.Accum Damage` (`self.Instant Damage`)))
  (if (> _output_get (`self.Max Damage`))
    (set `self.Accum Damage` (`self.Max Damage`))
    (`/Game/FirstPersonBP/Blueprints/FirstPersonCharacter.Change Health` (`self.Player`) (`self.Accum Damage`))))

(fn `UserConstructionScript`
  (bind _capsule (`self.Capsule`))
  (`SceneComponent.K2_SetWorldLocation` _capsule (+ (`KismetMathLibrary.MakeVector` 0.0 0.0 (`self.Laser Length`)) (`SceneComponent.K2_GetComponentLocation` _capsule)) false false)
  (`SceneComponent.K2_SetWorldTransform` _capsule (`KismetMathLibrary.MakeTransform` (.location (`SceneComponent.K2_GetComponentToWorld` _capsule)) (struct) (+ (.scale (`SceneComponent.K2_GetComponentToWorld` _capsule)) (`KismetMathLibrary.MakeVector` 0.0 0.0 (`self.Laser Scale`)))) false false))