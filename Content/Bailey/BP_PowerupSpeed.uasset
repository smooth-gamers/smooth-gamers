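; BP_PowerupSpeed is a pickup that temporarily boosts the first-person character's walk and crouch speeds on overlap.
; A game manager flag prevents stacking, so pickups touched during a boost stay in place.
; The actor hides and disables collision while a delay runs, then restores hardcoded speeds and clears the flag.
; The sound and noise event fire when the boost expires, just before the actor destroys itself.
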(event `self.AmmoCollision.OnComponentBeginOverlap`
  (params (OverlappedComponent :type "PrimitiveComponent Object Reference") (OtherActor :type "Actor Object Reference") (OtherComp :type "PrimitiveComponent Object Reference") (OtherBodyIndex :type Integer) (bFromSweep :type Boolean) (SweepResult :type "HitResult Structure (by ref)"))
  (bind _returnvalue (`self.K2_GetActorLocation`))
  ;[1 1 1] If player doesn't have a speed boost
  (bind _asfirst_person_character (cast `/Game/FirstPersonBP/Blueprints/FirstPersonCharacter` OtherActor))
  (bind _mygamemanager (`/Game/PublicStuff/MyFunctionLibrary.GetMyGameManager`))
  (if (not (`/Game/PublicStuff/MyGameManager.isSpeedBoosted` _mygamemanager))
    (set `/Game/PublicStuff/MyGameManager.isSpeedBoosted` true _mygamemanager)
    (bind _charactermovement (`Character.CharacterMovement` _asfirst_person_character))
    ;[1 1 1] Set boosted speeds
    (bind _output_get (set `CharacterMovementComponent.MaxWalkSpeed` (* (`MovementComponent.GetMaxSpeed` _charactermovement) (`self.SpeedMultiplier`)) _charactermovement))
    (set `CharacterMovementComponent.MaxWalkSpeedCrouched` (/ _output_get 2.0) _charactermovement)
    ;[1 1 1] Despawn and speed timer
    (`self.SetActorHiddenInGame` true)
    (`self.SetActorEnableCollision` false)
    (`KismetSystemLibrary.Delay` (`self.BoostDuration`))
    (set `CharacterMovementComponent.MaxWalkSpeed` 600.0 _charactermovement)
    (set `CharacterMovementComponent.MaxWalkSpeedCrouched` 300.0 _charactermovement)
    (set `/Game/PublicStuff/MyGameManager.isSpeedBoosted` false _mygamemanager)
    (`GameplayStatics.PlaySoundAtLocation` "/Game/Bailey/Sounds/Speed.Speed" _returnvalue (struct) 1.0 1.0 0.0 null null null) ; Play firing sound
    (`AISense_Hearing.ReportNoiseEvent` _returnvalue 1.0 self)
    (`self.K2_DestroyActor`)))

(fn `UserConstructionScript`)