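; Melee enemy character that damages the player on capsule hit or overlap and takes damage through ChangeEnemyHealth.
; Each tick it feeds health to a widget bar, turns the bar toward the player camera, and shows it when a camera line trace hits the enemy's healthbar collision.
; At zero health it removes the bar, ragdolls, disables capsule collision and rolls weighted chances to drop an SMG or shotgun pickup.
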(event `Ragdoll`
  (`PrimitiveComponent.SetSimulatePhysics` (`self.Mesh`) true))

(event `self.ReceiveTick`
  (params (DeltaSeconds :type "Float (single-precision)"))
  ;[1 1 1] Sets Health Value to widget
  (`self.Show Health bar`)
  (`self.Rotate Health bar`)
  (if (not (<= (`self.Health `) 0.0))
    (bind _aswidget_enemy_health (cast `/Game/UI/Widget_EnemyHealth` (`WidgetComponent.GetUserWidgetObject` (`self.Health bar`))))
    (bind _output_get (set `self.As Widget Enemy Health` _aswidget_enemy_health))
    (set `/Game/UI/Widget_EnemyHealth.Widget health` (/ (`self.Health `) 100.0) _output_get)))

(event `self.CapsuleComponent.OnComponentHit`
  (params (HitComponent :type "PrimitiveComponent Object Reference") (OtherActor :type "Actor Object Reference") (OtherComp :type "PrimitiveComponent Object Reference") (NormalImpulse :type "Vector Structure") (Hit :type "HitResult Structure (by ref)"))
  (if (== OtherActor (`GameplayStatics.GetPlayerCharacter` 0))
    (bind _asfirst_person_character (cast `/Game/FirstPersonBP/Blueprints/FirstPersonCharacter` OtherActor))
    (`/Game/FirstPersonBP/Blueprints/FirstPersonCharacter.Change Health` _asfirst_person_character -10.0)))

(event `self.CapsuleComponent.OnComponentBeginOverlap`
  (params (OverlappedComponent :type "PrimitiveComponent Object Reference") (OtherActor :type "Actor Object Reference") (OtherComp :type "PrimitiveComponent Object Reference") (OtherBodyIndex :type Integer) (bFromSweep :type Boolean) (SweepResult :type "HitResult Structure (by ref)"))
  (if (== OtherActor (`GameplayStatics.GetPlayerCharacter` 0))
    (bind _asfirst_person_character (cast `/Game/FirstPersonBP/Blueprints/FirstPersonCharacter` OtherActor))
    (`/Game/FirstPersonBP/Blueprints/FirstPersonCharacter.Change Health` _asfirst_person_character -10.0)))

(fn `Change Enemy Health`
  (params (`Incoming Damage` :type "Float (double-precision)"))
  (`self.Set Enemy Health` (- (`self.Health `) `Incoming Damage`)))

(fn `Rotate Health bar`
  (bind _health_bar (`self.Health bar`))
  (if (not (<= (`self.Health `) 0.0))
    (bind _asfirst_person_character (cast `/Game/FirstPersonBP/Blueprints/FirstPersonCharacter` (`GameplayStatics.GetPlayerPawn` 0)))
    (`SceneComponent.K2_SetWorldRotation` _health_bar (`KismetMathLibrary.FindLookAtRotation` (`SceneComponent.K2_GetComponentLocation` _health_bar) (`SceneComponent.K2_GetComponentLocation` (`/Game/FirstPersonBP/Blueprints/FirstPersonCharacter.FirstPersonCamera` _asfirst_person_character))) false false)))

(fn `Set Enemy Health`
  (params (Health :type "Float (double-precision)"))
  (bind _returnvalue (`KismetMathLibrary.Conv_VectorToTransform` (`self.K2_GetActorLocation`)))
  (bind _output_get (set `self.Health ` Health))
  (if (> _output_get 100.0)
    (set `self.Health ` 100.0))
  (if (<= _output_get 0.0)
    (`ActorComponent.K2_DestroyComponent` (`self.Health bar`))
    (`self.Ragdoll`)
    (`PrimitiveComponent.SetCollisionEnabled` (`self.CapsuleComponent`) "NoCollision")
    (if (`KismetMathLibrary.RandomBoolWithWeight` (`self.SMGDROPCHANCE`))
      (`|SpawnActorFromClass` "/Game/Johnathan/BPs/SMGPickup.SMGPickup_C" _returnvalue "AlwaysSpawn" "OverrideRootScale" null null)
      (elif (`KismetMathLibrary.RandomBoolWithWeight` (`self.ShotGunChance`))
        (`|SpawnActorFromClass` "/Game/Johnathan/BPs/SHoutGunPickup.SHoutGunPickup_C" _returnvalue "AlwaysSpawn" "OverrideRootScale" null null)))))

(fn `Show Health bar`
  (bind _health_bar (`self.Health bar`))
  (if (not (<= (`self.Health `) 0.0))
    (bind _asfirst_person_character (cast `/Game/FirstPersonBP/Blueprints/FirstPersonCharacter` (`GameplayStatics.GetPlayerPawn` 0)))
    (bind _outactors (`GameplayStatics.GetAllActorsOfClass` "/Game/FirstPersonBP/Blueprints/FirstPersonCharacter.FirstPersonCharacter_C"))
    (bind _firstpersoncamera (`/Game/FirstPersonBP/Blueprints/FirstPersonCharacter.FirstPersonCamera` _asfirst_person_character))
    (bind _returnvalue (`SceneComponent.K2_GetComponentLocation` _firstpersoncamera))
    (bind (_outhit _returnvalue_2) (`KismetSystemLibrary.LineTraceSingle` _returnvalue (+ _returnvalue (* (`SceneComponent.GetForwardVector` _firstpersoncamera) 50000.0)) "TraceTypeQuery2" false _outactors "None" false (struct :`R` 1.0 :`A` 1.0) (struct :`G` 1.0 :`A` 1.0) 1.0))
    (if _returnvalue_2
      (if (== (`.HitComponent` (`GameplayStatics.BreakHitResult` _outhit)) (`self.ShowHealthbar_Collision`))
        (`SceneComponent.SetVisibility` _health_bar true false)
        (else
          (`SceneComponent.SetVisibility` _health_bar false false))))))

(fn `UserConstructionScript`)